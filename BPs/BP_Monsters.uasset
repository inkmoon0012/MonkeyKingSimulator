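; BP_Monsters is a melee monster Character with entry events for a normal attack, a charged skill and target lock-on.
; MonsterSkill1 plays a charge montage, then a release montage, gated by a cooldown and hit state.
; Lock-on snaps yaw toward the target and toggles orient-to-movement.
; The normal-attack combo and player hit, block and stun logic are disconnected, so both overlap events and EnemyAttack currently do nothing.
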(event OnComponentBeginOverlap(CapsuleComponent)
  (params (OverlappedComponent :type Primitive%20Component%20Object%20Reference) (OtherActor :type Actor%20Object%20Reference) (OtherComp :type Primitive%20Component%20Object%20Reference) (OtherBodyIndex :type Integer) (bFromSweep :type Boolean) (SweepResult :type Hit%20Result%20Structure%20%28by%20ref%29))
  ;[1 1 1] OnHit
)

(event OnComponentBeginOverlap(WeaponCapsule)
  (params (OverlappedComponent :type Primitive%20Component%20Object%20Reference) (OtherActor :type Actor%20Object%20Reference) (OtherComp :type Primitive%20Component%20Object%20Reference) (OtherBodyIndex :type Integer) (bFromSweep :type Boolean) (SweepResult :type Hit%20Result%20Structure%20%28by%20ref%29))
  ;[1 1 1] Blocked by Player
)

(event EventEnemyAttack
  ;[1 1 1] NormalAttack
  (|NormalAttack) ; enters at Execute2
)

(event EventEnemySkill1
  ;[1 1 1] Skill1
  (|MonsterSkill1) ; enters at Exe2
)

(event EventLockon
  (params (TargetLocked :type Actor%20Object%20Reference) (Lock%20On/Off :type Boolean))
  (bind _returnvalue (Transformation|GetActorRotation))
  ;[1 1 1] LockOn
  (if Lock%20On/Off
    (Utilities|IsValid TargetLocked
      (:Is%20Valid
        (Variables|/Script/Engine.CharacterMovementComponent|SetbOrientRotationToMovement (Variables|Character|GetCharacterMovement) false)
        (Transformation|SetActorRotation (Math|Rotator|MakeRotator (.roll _returnvalue) (.pitch _returnvalue) (.yaw (Math|Rotator|FindLookatRotation (Transformation|GetActorLocation) (Transformation|GetActorLocation TargetLocked))))))
      (:Is%20Not%20Valid
        (Variables|/Script/Engine.CharacterMovementComponent|SetbOrientRotationToMovement (Variables|Character|GetCharacterMovement) true :!label _label)))
    (else
      (goto _label))))

(fn ConstructionScript
  (|CallParentFunction))